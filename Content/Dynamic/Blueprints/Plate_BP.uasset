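; Plate_BP is a clickable, colored plate actor that the player selects for control.
; On BeginPlay it prints its PlateColor enum and applies the matching blue, yellow or red material to its Plate component.
; A click casts the first player controller to PlateController_BP and registers this plate as the controlled one.
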(event `self.ReceiveActorOnClicked`
  (params (ButtonPressed :type "Key Structure"))
  (bind _asplate_controller_bp (cast `/Game/Dynamic/Blueprints/PlateController_BP` (`GameplayStatics.GetPlayerController` 0)))
  (`PlateController.SetControlledPlate` _asplate_controller_bp self))

(event `self.ReceiveBeginPlay`
  (bind _platecolor (`self.PlateColor`))
  (`KismetSystemLibrary.PrintString` (`|GetEnumeratorNameAsString` _platecolor))
  (`PrimitiveComponent.SetMaterial` (`self.Plate`) 0 (select `EPlateColor` _platecolor :`Blue` "/Engine/BasicShapes/PlateBlue.PlateBlue" :`Yellow` "/Engine/BasicShapes/PlateYellow.PlateYellow" :`Red` "/Engine/BasicShapes/PlateRed.PlateRed" :!type "MaterialInterface Object Reference")))

(fn `UserConstructionScript`)