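; PlateController_BP is an input-driven controller for moving plates in a plates-and-blocks puzzle game.
; The four directional input actions each call a matching MovePlate function, none of which is defined in this graph.
; After every move, all paths converge to ask PlatesAndBlocksGameModeBase whether the game is complete, and if so show a Congratulation widget on the viewport.
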(event `InputAction|MoveUp`
  (params (Key :type "Key Structure"))
  (:`Pressed`
    (`self.MovePlateUp`)
    (bind _asplates_and_blocks_game_mode_base (cast `PlatesAndBlocksGameModeBase` (`GameplayStatics.GetGameMode`) :!label _label))
    (bind _returnvalue (`PlatesAndBlocksGameModeBase.CheckGameCompletion` _asplates_and_blocks_game_mode_base))
    (if _returnvalue
      (bind _returnvalue_2 (`|CreateWidget` "/Game/Dynamic/Widgets/Congratulation.Congratulation_C"))
      (`UserWidget.AddToViewport` _returnvalue_2 0))))

(event `InputAction|MoveDown`
  (params (Key :type "Key Structure"))
  (:`Pressed`
    (`self.MovePlateDown`)
    (goto _label)))

(event `InputAction|MoveLeft`
  (params (Key :type "Key Structure"))
  (:`Pressed`
    (`self.MovePlateLeft`)
    (goto _label)))

(event `InputAction|MoveRight`
  (params (Key :type "Key Structure"))
  (:`Pressed`
    (`self.MovePlateRight`)
    (goto _label)))

(fn `UserConstructionScript`)